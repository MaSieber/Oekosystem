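; Player character Blueprint for WorldDiscovery, built around a magnetism ability that holds, pushes and spins objects.
; Magnetic input toggles the effect and audio, with release cleanup shared by OnReset, while push and spin target the active object, with shields spinning faster.
; Dynamic materials drive a timed damage flash, followed by Reset, and the magnetic wave's rotation.
; It also creates the player HUD and handles pause, god-mode cheat and data-table level cycling.
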(event Custom|OnDamageDelayOver_Event
  ;[1 1 1] Comment
  (Class|KismetSystemLibrary|ClearTimerHandle (stale EventOnDamaged _returnvalue_2))
  (Class|NewWorldDiscoveryCharacter|Reset)
  (bind _returnvalue (Rendering|Material|CreateDynamicMaterialInstance (Variables|Character|GetMesh) 0 "/Game/Player_Char/Materials/T_DIFFUSE_CHAR_TEST_02_Mat.T_DIFFUSE_CHAR_TEST_02_Mat" :!class /Script/Engine.PrimitiveComponent))
  (Rendering|Material|SetScalarParameterValue _returnvalue "Damage" 0.0 :!class /Script/Engine.MaterialInstanceDynamic))

(event EventBeginPlay
  ;[1 1 1] Set Player UI
  (bind _asworld_discovery_player_controller (Utilities|Casting|CastToWorldDiscoveryPlayerController (Game|GetPlayerController 0)))
  (Game|Player|SetViewTargetwithBlend _asworld_discovery_player_controller self 0.0 "VTBlend_Linear" 0.0 false)
  (bind _returnvalue (UserInterface|CreateWidget "/Game/UI/UI_Player.UI_Player_C" _asworld_discovery_player_controller))
  (UserInterface|Viewport|AddtoViewport _returnvalue 0))

(event EventOnRotateAround
  (params (val :type Float%20%28single-precision%29))
  ;[1 1 1] Input
  ;;[1 1 1] Rotate Around
  (bind _returnvalue (Class|NewWorldDiscoveryCharacter|GetPlayerDegree))
  (if (!= _returnvalue 0)
    (if (Variables|/Script/NewWorldDiscovery.PlayerDegree|GetbParticleRotation _returnvalue)
      (bind _asbp_player_xdegree (Utilities|Casting|CastToBP_PlayerXDegree _returnvalue))
      (bind _returnvalue_2 (Rendering|Material|CreateDynamicMaterialInstance (Variables|/Script/NewWorldDiscovery.PlayerXDegree|GetmagneticWaveSingle _asbp_player_xdegree) 1 "/Game/PFX/Materials/M_MagneticWaveTest.M_MagneticWaveTest" :!class /Script/Engine.PrimitiveComponent))
      (bind _output_get (Variables|Default|SetCurrentRotation (Math|Float|%(Float) (+ (Variables|Default|GetCurrentRotation) (/ val -1e+02)) 1.0)))
      (Rendering|Material|SetScalarParameterValue _returnvalue_2 "Angle" _output_get :!class /Script/Engine.MaterialInstanceDynamic))))

(event EventOnDamaged
  ;[1 1 1] Comment
  (bind _returnvalue (Rendering|Material|CreateDynamicMaterialInstance (Variables|Character|GetMesh) 0 "/Game/Player_Char/Materials/T_DIFFUSE_CHAR_TEST_02_Mat.T_DIFFUSE_CHAR_TEST_02_Mat" :!class /Script/Engine.PrimitiveComponent))
  (Rendering|Material|SetScalarParameterValue _returnvalue "Damage" 1.0 :!class /Script/Engine.MaterialInstanceDynamic)
  (bind _returnvalue_2 (Utilities|Time|SetTimerbyEvent (delegate Custom|OnDamageDelayOver_Event) 0.1)))

(event EventOnReset
  ;[1 1 1] Input
  ;;[1 1 1] Magnetic Effect
  (Class|NewWorldDiscoveryCharacter|EmptyHoldingObjects)
  (Class|NewWorldDiscoveryCharacter|DisableMagnetic)
  (Variables|Default|SetCurrentRotation 0.0)
  (Audio|Components|Audio|Stop (Variables|Default|GetAudio)))

(event EventOnCreate
  (Components|Activation|Activate (Variables|Default|GetPFX_Creation) false))

(event Input|ActionEvents|InputActionMagnetic
  (params (Key :type Key%20Structure :default "AnyKey"))
  (bind _audio (Variables|Default|GetAudio))
  ;[1 1 1] Input
  ;;[1 1 1] Magnetic Effect
  (:Pressed
    (Class|NewWorldDiscoveryCharacter|EnableMagnetic)
    (Audio|Components|Audio|Play _audio 0.0))
  (:Released
    (for _array_element (Variables|Default|GetHoldingObjects)
      (Class|BaseMagnetic|TriggerMagneticStop _array_element))
    (Class|NewWorldDiscoveryCharacter|EmptyHoldingObjects)
    (Class|NewWorldDiscoveryCharacter|DisableMagnetic)
    (Variables|Default|SetCurrentRotation 0.0)
    (Audio|Components|Audio|Stop _audio)))

(event Input|ActionEvents|InputActionPause
  (params (Key :type Key%20Structure :default "AnyKey"))
  ;[1 1 1] Input
  ;;[1 1 1] Pause
  (:Pressed
    (if (Variables|Default|GetIsPaused)
      (Widget|RemovefromParent (stale _returnvalue))
      (bind _output_get (Variables|Default|SetIsPaused false))
      (Game|SetGamePaused _output_get)
      (else
        (bind _asbp_world_discovery_player_ctrl (Utilities|Casting|CastToBP_WorldDiscoveryPlayerCtrl (Game|GetPlayerController 0)))
        (bind _returnvalue (UserInterface|CreateWidget "/Game/UI/UI_Pause.UI_Pause_C" _asbp_world_discovery_player_ctrl))
        (UserInterface|Viewport|AddtoViewport _returnvalue 0)
        (Input|SetInputModeGameandUI _asbp_world_discovery_player_ctrl _returnvalue false true)
        (bind _returnvalue_2 (Game|SetGamePaused true))
        (Variables|Default|SetIsPaused _returnvalue_2)))))

(event Input|ActionEvents|InputActionMapSwitch
  (params (Key :type Key%20Structure :default "AnyKey"))
  ;[1 1 1] Input
  ;;[1 1 1] CheatKey
  (:Pressed
    (bind _asbp_world_discovery_game_instance (Utilities|Casting|CastToBP_WorldDiscoveryGameInstance (Game|GetGameInstance))
      (:then
        (bind _outrownames (DataTable|GetDataTableRowNames "/Game/Data/Levels.Levels"))
        (Development|PrintString (Utilities|String|ToString(Integer) (+ (Variables|/Script/NewWorldDiscovery.WorldDiscoveryGameInstance|GetCurrentMapIndex _asbp_world_discovery_game_instance) 1)))
        (if (> (Utilities|Array|Length _outrownames) (+ (Variables|/Script/NewWorldDiscovery.WorldDiscoveryGameInstance|GetCurrentMapIndex _asbp_world_discovery_game_instance) 1))
          (Variables|/Script/NewWorldDiscovery.WorldDiscoveryGameInstance|SetCurrentMapIndex _asbp_world_discovery_game_instance (+ (Variables|/Script/NewWorldDiscovery.WorldDiscoveryGameInstance|GetCurrentMapIndex _asbp_world_discovery_game_instance) 1))
          (else
            (Variables|/Script/NewWorldDiscovery.WorldDiscoveryGameInstance|SetCurrentMapIndex _asbp_world_discovery_game_instance 0)))
        (bind _returnvalue (Utilities|GetDataTableRow "/Game/Data/Levels.Levels" (Utilities|Array|Get(acopy) _outrownames (Variables|/Script/NewWorldDiscovery.WorldDiscoveryGameInstance|GetCurrentMapIndex _asbp_world_discovery_game_instance)))
          (:then
            (Game|OpenLevel(byName) (Utilities|String|StringToName (.Tag (Utilities|Struct|BreakGameplayTagTableRow _returnvalue)))))))
      (:CastFailed
        (Development|PrintString "Hello")))))

(event Input|ActionEvents|InputActionCheatKey
  (params (Key :type Key%20Structure :default "AnyKey"))
  ;[1 1 1] Input
  ;;[1 1 1] CheatKey
  (:Pressed
    (Class|NewWorldDiscoveryCharacter|Godmode)))

(event Input|ActionEvents|InputActionMagneticPush
  (params (Key :type Key%20Structure :default "AnyKey"))
  ;[1 1 1] Input
  ;;[1 1 1] Push
  (:Pressed
    (bind _returnvalue (Class|NewWorldDiscoveryCharacter|GetActiveObject))
    (if (not (== _returnvalue 0))
      (Class|MagneticBox|TriggerMagneticPush _returnvalue)
      (Audio|PlaySoundatLocation "/Game/Sound/SFX/Magnetismus_abstossen_edit.Magnetismus_abstossen_edit" (Transformation|GetActorLocation)))))

(event Input|ActionEvents|InputActionSpinPulled
  (params (Key :type Key%20Structure :default "AnyKey"))
  ;[1 1 1] Input
  ;;[1 1 1] Spin
  (:Pressed
    (Variables|Default|SetTempVelocity 5e+01)
    (bind _returnvalue (Class|NewWorldDiscoveryCharacter|GetActiveObject :!label _label))
    (if (not (== _returnvalue 0))
      (bind _asbp_magnetic_shield (Utilities|Casting|CastToBP_MagneticShield _returnvalue)
        (:then
          (Variables|/Script/NewWorldDiscovery.BaseMagnetic|SetRotationVelocity _asbp_magnetic_shield (* 2.5 (Variables|Default|GetTempVelocity))))
        (:CastFailed
          (Variables|/Script/NewWorldDiscovery.BaseMagnetic|SetRotationVelocity _returnvalue (Variables|Default|GetTempVelocity))))))
  (:Released
    (Variables|Default|SetTempVelocity 0.0)
    (goto _label)))

(fn ConstructionScript)