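; Background decoration actor for a rotating gear (Zahnrad) in the scenery, with optional looping or one-shot audio.
; When Active, it starts its audio on BeginPlay if Sound is enabled.
; Each tick it advances an angle by AlphaSpeed, wrapped at 360 degrees, and applies it as the roll of the gear plane's relative rotation.
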(event EventBeginPlay
  (if (Variables|Default|GetbActive)
    (if (Variables|Default|GetbSound)
      (Audio|Components|Audio|Play (Variables|Default|GetAudio) 0.0))))

(event EventTick
  (params (DeltaSeconds :type Float%20%28single-precision%29))
  (if (Variables|Default|GetbActive)
    (bind _output_get (Variables|Default|SetAlpha (Math|Float|%(Float) (+ (* DeltaSeconds (Variables|Default|GetAlphaSpeed)) (Variables|Default|GetAlpha)) 3.6e+02)))
    (Transformation|SetRelativeRotation (Variables|Default|GetZahnradPlane) (Math|Rotator|MakeRotator _output_get 0.0 0.0) false false)))

(fn ConstructionScript)