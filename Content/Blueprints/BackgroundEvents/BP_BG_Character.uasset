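; BP_BG_Character is a background event Blueprint that continuously spins a gear plane component (ZahnradPlane).
; While Active is set, Tick advances Alpha by AlphaSpeed scaled with delta time, wrapping it within a full turn.
; Alpha is then applied as the plane's relative yaw, with pitch and roll held at zero.
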(event EventTick
  (params (DeltaSeconds :type Float%20%28single-precision%29))
  (if (Variables|Default|GetbActive)
    (bind _output_get (Variables|Default|SetAlpha (Math|Float|%(Float) (+ (* DeltaSeconds (Variables|Default|GetAlphaSpeed)) (Variables|Default|GetAlpha)) 3.6e+02)))
    (Transformation|SetRelativeRotation (Variables|Default|GetZahnradPlane) (Math|Rotator|MakeRotator 0.0 0.0 _output_get) false false)))

(fn ConstructionScript)