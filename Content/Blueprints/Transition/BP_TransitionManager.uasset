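; BP_TransitionManager switches between levels, taking the level list and current map index from BP_WorldDiscoveryGameInstance.
; OnLoadNewLevel picks the next level, saves its index, then either stream-loads it or opens it by name, depending on LoadAsync.
; An optional UI_SplashScreen covers the load.
; OnUnloadOldLevel acts only in async mode, resolving the last row's level, writing that index back and unloading the streamed level.
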(event EventOnUnloadOldLevel
  (if (Variables|Default|GetbLoadAsync)
    (bind _asbp_world_discovery_game_instance (Utilities|Casting|CastToBP_WorldDiscoveryGameInstance (Game|GetGameInstance)))
    (bind (_levels _currentindex) (CallFunction|GetLevels _asbp_world_discovery_game_instance))
    (bind (_tag _newindex) (CallFunction|GetDataTableLastRowTag _levels _currentindex))
    (Variables|/Script/NewWorldDiscovery.WorldDiscoveryGameInstance|SetCurrentMapIndex _asbp_world_discovery_game_instance _newindex)
    (Game|UnloadStreamLevel(byName) _tag)))

(event EventOnLoadNewLevel
  (bind _asbp_world_discovery_game_instance (Utilities|Casting|CastToBP_WorldDiscoveryGameInstance (Game|GetGameInstance)))
  (bind (_levels _currentindex) (CallFunction|GetLevels _asbp_world_discovery_game_instance))
  (bind (_tag _newindex) (CallFunction|GetDataTableNextRowTag _levels _currentindex))
  (Variables|/Script/NewWorldDiscovery.WorldDiscoveryGameInstance|SetCurrentMapIndex _asbp_world_discovery_game_instance _newindex)
  (if (Variables|Default|GetbLoadingScreen)
    (bind _asworld_discovery_player_controller (Utilities|Casting|CastToWorldDiscoveryPlayerController (Game|GetPlayerController 0)))
    (bind _returnvalue (UserInterface|CreateWidget "/Game/UI/UI_SplashScreen.UI_SplashScreen_C" _asworld_discovery_player_controller))
    (bind _output_get (Variables|Default|SetUserWidget _returnvalue))
    (UserInterface|Viewport|AddtoViewport _output_get 0))
  (if (Variables|Default|GetbLoadAsync)
    (Game|LoadStreamLevel(byName) _tag true)
    (Widget|RemovefromParent (Variables|Default|GetUserWidget))
    (else
      (Game|OpenLevel(byName) _tag)
      (Widget|RemovefromParent (Variables|Default|GetUserWidget)))))

(fn ConstructionScript)