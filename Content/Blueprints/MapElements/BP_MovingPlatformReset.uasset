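; BP_MovingPlatformReset is a map element with a reset mesh that plays glow feedback when its OnReset event fires.
; A Done flag ignores repeat calls until the sequence finishes.
; Each reset creates a dynamic M_Generator material instance, briefly brightens the button emissive, then plays the Triggering timeline to drive the main emissive strength.
; The file itself contains no platform movement logic, only the visual response.
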(event EventOnReset
  (if (Variables|Default|GetDone)
    (Variables|Default|SetDone false)
    (bind _returnvalue (Rendering|Material|CreateDynamicMaterialInstance (Variables|Default|GetResetMesh) 0 "/Game/MapElements/Materials/M_Generator.M_Generator" :!class /Script/Engine.PrimitiveComponent))
    (Rendering|Material|SetScalarParameterValue _returnvalue "EmissiveStrengthButton" 2e+01 :!class /Script/Engine.MaterialInstanceDynamic)
    (Utilities|FlowControl|Delay 0.5)
    (Rendering|Material|SetScalarParameterValue _returnvalue "EmissiveStrengthButton" 1.0 :!class /Script/Engine.MaterialInstanceDynamic)
    (bind _newtrack_0 (Timeline|Triggering PlayFromStart)
      (:Update
        (Rendering|Material|SetScalarParameterValue _returnvalue "EmissiveStrength" (+ (* _newtrack_0 1e+02) 5.0) :!class /Script/Engine.MaterialInstanceDynamic))
      (:Finished
        (Variables|Default|SetDone true)))))

(fn ConstructionScript)