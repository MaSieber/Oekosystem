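; BP_MagneticEnergyTransfer is a magnetic energy-carrier actor that can be created, charged, discharged and destroyed.
; Powering up and down toggles the Powered flag, flash effects, sounds and emissive material parameters, with an energy-loss particle effect on discharge.
; OnCreate reuses the no-energy setup, then a timeline dissolves the mesh in before enabling physics and overlaps.
; OnDestroying runs a second dissolve timeline, then destroys the actor.
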(event EventOnPoweringDown
  (bind _magneticmesh (Variables|Default|GetMagneticMesh))
  (Variables|Default|SetPoweringDown true)
  (Audio|PlaySoundatLocation "/Game/Sound/SFX/KugelEntladen.KugelEntladen" (Transformation|GetActorLocation))
  (if (Variables|Default|GetPowered)
    (Components|Activation|Activate (Variables|Default|GetPFX_EnergyLos) true)
    ;[1 1 1] Initialize/NoEnergy
    (Components|Activation|Deactivate (Variables|Default|GetFlash))
    (Components|Activation|Deactivate (Variables|Default|GetFlash2))
    (Components|Activation|Deactivate (Variables|Default|GetFlash3))
    (bind _returnvalue (Rendering|Material|CreateDynamicMaterialInstance (Variables|Default|GetMagneticMesh) 0 "/Game/MapElements/Materials/MI_EnergyTransfer_Adv.MI_EnergyTransfer_Adv" :!class /Script/Engine.PrimitiveComponent))
    (Rendering|Material|SetScalarParameterValue _returnvalue "EmissiveStrength" 0.0 :!class /Script/Engine.MaterialInstanceDynamic)
    (Rendering|Material|SetScalarParameterValue _returnvalue "SaturateRate" 4.0 :!class /Script/Engine.MaterialInstanceDynamic)
    (Rendering|Material|SetScalarParameterValue _returnvalue "FringeSize" 3.0 :!class /Script/Engine.MaterialInstanceDynamic)
    (Variables|Default|SetPowered false)
    (if (not (Variables|Default|GetPoweringDown))
      (Rendering|Material|SetScalarParameterValue _returnvalue "DisolveStrength" 1.0 :!class /Script/Engine.MaterialInstanceDynamic)
      (Audio|PlaySoundatLocation "/Game/Sound/SFX/Obejkt_erstellen.Obejkt_erstellen" (Transformation|GetActorLocation))
      ;[1 1 1] Spawn
      (bind _emissivepower (Timeline|Timeline_0 PlayFromStart)
        (:Update
          (Rendering|Material|SetScalarParameterValue _returnvalue "DisolveStrength" (Math|Float|Clamp(Float) (- 1.0 _emissivepower)) :!class /Script/Engine.MaterialInstanceDynamic))
        (:Finished
          (Physics|SetSimulatePhysics _magneticmesh true)
          (Variables|/Script/Engine.PrimitiveComponent|SetbGenerateOverlapEvents _magneticmesh true)
          (Rendering|Material|SetScalarParameterValue _returnvalue "FringeSize" 0.0 :!class /Script/Engine.MaterialInstanceDynamic))))))

(event EventOnCreate
  (bind _magneticmesh (Variables|Default|GetMagneticMesh))
  (Components|Activation|Activate (Variables|Default|GetPFX_Sparks) true)
  (Variables|Default|SetPoweringDown false)
  ;[1 1 1] Initialize/NoEnergy
  (Components|Activation|Deactivate (Variables|Default|GetFlash))
  (Components|Activation|Deactivate (Variables|Default|GetFlash2))
  (Components|Activation|Deactivate (Variables|Default|GetFlash3))
  (bind _returnvalue (Rendering|Material|CreateDynamicMaterialInstance (Variables|Default|GetMagneticMesh) 0 "/Game/MapElements/Materials/MI_EnergyTransfer_Adv.MI_EnergyTransfer_Adv" :!class /Script/Engine.PrimitiveComponent))
  (Rendering|Material|SetScalarParameterValue _returnvalue "EmissiveStrength" 0.0 :!class /Script/Engine.MaterialInstanceDynamic)
  (Rendering|Material|SetScalarParameterValue _returnvalue "SaturateRate" 4.0 :!class /Script/Engine.MaterialInstanceDynamic)
  (Rendering|Material|SetScalarParameterValue _returnvalue "FringeSize" 3.0 :!class /Script/Engine.MaterialInstanceDynamic)
  (Variables|Default|SetPowered false)
  (if (not (Variables|Default|GetPoweringDown))
    (Rendering|Material|SetScalarParameterValue _returnvalue "DisolveStrength" 1.0 :!class /Script/Engine.MaterialInstanceDynamic)
    (Audio|PlaySoundatLocation "/Game/Sound/SFX/Obejkt_erstellen.Obejkt_erstellen" (Transformation|GetActorLocation))
    ;[1 1 1] Spawn
    (bind _emissivepower (Timeline|Timeline_0 PlayFromStart)
      (:Update
        (Rendering|Material|SetScalarParameterValue _returnvalue "DisolveStrength" (Math|Float|Clamp(Float) (- 1.0 _emissivepower)) :!class /Script/Engine.MaterialInstanceDynamic))
      (:Finished
        (Physics|SetSimulatePhysics _magneticmesh true)
        (Variables|/Script/Engine.PrimitiveComponent|SetbGenerateOverlapEvents _magneticmesh true)
        (Rendering|Material|SetScalarParameterValue _returnvalue "FringeSize" 0.0 :!class /Script/Engine.MaterialInstanceDynamic)))))

(event EventOnPoweringUp
  (if (not (Variables|Default|GetPowered))
    (Audio|PlaySoundatLocation "/Game/Sound/SFX/KugelLaden.KugelLaden" (Transformation|GetActorLocation))
    ;[1 1 1] Activate
    (Components|Activation|Activate (Variables|Default|GetFlash3) true)
    (Components|Activation|Activate (Variables|Default|GetFlash2) true)
    (Components|Activation|Activate (Variables|Default|GetFlash) true)
    (bind _returnvalue (Rendering|Material|CreateDynamicMaterialInstance (Variables|Default|GetMagneticMesh) 0 "/Game/MapElements/Materials/M_EnergyTransfer.M_EnergyTransfer" :!class /Script/Engine.PrimitiveComponent))
    (Rendering|Material|SetScalarParameterValue _returnvalue "EmissiveStrength" 1.5e+02 :!class /Script/Engine.MaterialInstanceDynamic)
    (Rendering|Material|SetScalarParameterValue _returnvalue "SaturateRate" 2.0 :!class /Script/Engine.MaterialInstanceDynamic)
    (Variables|Default|SetPowered true)))

(event EventOnDestroying
  (bind _emissivepower (Timeline|Timeline_1 PlayFromStart)
    (:Update
      (bind _returnvalue (Rendering|Material|CreateDynamicMaterialInstance (Variables|Default|GetMagneticMesh) 0 "/Game/MapElements/Materials/M_EnergyTransfer.M_EnergyTransfer" :!class /Script/Engine.PrimitiveComponent))
      (Rendering|Material|SetScalarParameterValue _returnvalue "DisolveStrength" (Math|Float|Clamp(Float) _emissivepower) :!class /Script/Engine.MaterialInstanceDynamic))
    (:Finished
      (Actor|DestroyActor))))

(fn ConstructionScript)