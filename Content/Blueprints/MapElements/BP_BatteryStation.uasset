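; BP_BatteryStation is a map element that animates the glow of its battery mesh when energy rises or falls.
; Each energy event creates a dynamic instance of an emissive test material and runs a timeline that drives its EmissiveStrength parameter.
; OnEnergyFall plays the fade only if the current strength is above a threshold, while OnEnergyRise always plays the fade-in.
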(event EventOnEnergyFall
  (bind _returnvalue (Rendering|Material|CreateDynamicMaterialInstance (Variables|Default|GetBatteryMesh) 0 "/Game/Test/M_EmissionTest.M_EmissionTest" :!class /Script/Engine.PrimitiveComponent))
  (bind _returnvalue_2 (Rendering|Material|GetScalarParameterValue _returnvalue "EmissiveStrength" :!class /Script/Engine.MaterialInstanceDynamic))
  (if (not (<= _returnvalue_2 1.0))
    (bind _emission (Timeline|EmissionFade PlayFromStart)
      (:Update
        (Rendering|Material|SetScalarParameterValue _returnvalue "EmissiveStrength" (* _emission 1e+01) :!class /Script/Engine.MaterialInstanceDynamic)))))

(event EventOnEnergyRise
  (bind _returnvalue (Rendering|Material|CreateDynamicMaterialInstance (Variables|Default|GetBatteryMesh) 0 "/Game/Test/M_EmissionTest.M_EmissionTest" :!class /Script/Engine.PrimitiveComponent))
  (bind _emission (Timeline|EmissionFadeIn PlayFromStart)
    (:Update
      (Rendering|Material|SetScalarParameterValue _returnvalue "EmissiveStrength" (* _emission 1e+01) :!class /Script/Engine.MaterialInstanceDynamic))))

(fn ConstructionScript)