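; BP_MagneticEnergyProvider is a magnetic energy provider map element that dissolves in when created and dissolves out when destroyed.
; On creation, a timeline lowers the DisolveStrength parameter of M_EnergyProvider on MagneticMesh, then enables physics simulation on the mesh.
; On destruction, a second timeline drives that parameter from its own curve and destroys the actor when finished.
; Each timeline update creates a new dynamic material instance rather than reusing one.
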(event EventOnCreate
  (bind _magneticmesh (Variables|Default|GetMagneticMesh))
  (bind _returnvalue (Rendering|Material|CreateDynamicMaterialInstance (Variables|Default|GetMagneticMesh) 0 "/Game/MapElements/Materials/M_EnergyProvider.M_EnergyProvider" :!class /Script/Engine.PrimitiveComponent))
  (Rendering|Material|SetScalarParameterValue _returnvalue "DisolveStrength" 1.0 :!class /Script/Engine.MaterialInstanceDynamic)
  (bind _emissivepower (Timeline|Timeline_0 PlayFromStart)
    (:Update
      (bind _returnvalue_2 (Rendering|Material|CreateDynamicMaterialInstance _magneticmesh 0 "/Game/MapElements/Materials/M_EnergyProvider.M_EnergyProvider" :!class /Script/Engine.PrimitiveComponent))
      (Rendering|Material|SetScalarParameterValue _returnvalue_2 "DisolveStrength" (Math|Float|Clamp(Float) (- 1.0 _emissivepower)) :!class /Script/Engine.MaterialInstanceDynamic))
    (:Finished
      (Physics|SetSimulatePhysics _magneticmesh true))))

(event EventOnDestroying
  (bind _emissivepower (Timeline|DisolveFadeInOut PlayFromStart)
    (:Update
      (bind _returnvalue (Rendering|Material|CreateDynamicMaterialInstance (Variables|Default|GetMagneticMesh) 0 "/Game/MapElements/Materials/M_EnergyProvider.M_EnergyProvider" :!class /Script/Engine.PrimitiveComponent))
      (Rendering|Material|SetScalarParameterValue _returnvalue "DisolveStrength" (Math|Float|Clamp(Float) _emissivepower) :!class /Script/Engine.MaterialInstanceDynamic))
    (:Finished
      (Actor|DestroyActor))))

(fn ConstructionScript)