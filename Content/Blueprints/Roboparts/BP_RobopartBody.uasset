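; Robot body part that magnetically pulls leg parts into its left and right attachment points.
; Each point's collider overlap accepts only its matching leg, triggers its magnetic stop and starts pulling; only the left leg has gravity disabled.
; Tick drives the single stored part by setting its physics velocity toward the collider, scaled by distance.
; Pulling ends within two units, with no attachment step here, and debug prints trace the process.
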(event OnComponentBeginOverlap(LeftLegPointCollider)
  (params (OtherActor :type Actor%20Object%20Reference) (OtherComp :type Primitive%20Component%20Object%20Reference) (OtherBodyIndex :type Integer) (bFromSweep :type Boolean) (SweepResult :type Hit%20Result%20Structure%20%28by%20ref%29))
  (Development|PrintString "left leg collider")
  (bind _asrobopart_left_leg (Utilities|Casting|CastToRobopartLeftLeg OtherActor))
  (bind _output_get (Variables|Default|SetBaseRoboPart _asrobopart_left_leg))
  (Variables|Default|SetCollider (Variables|Default|GetLeftLegPointCollider))
  (Development|PrintString "is left leg")
  (Class|BaseMagnetic|TriggerMagneticStop _output_get)
  (Physics|SetEnableGravity (Variables|/Script/NewWorldDiscovery.BaseMagnetic|GetMagneticMesh _output_get) false)
  (Variables|Default|SetPulling true))

(event OnComponentBeginOverlap(RightLegPointCollider)
  (params (OtherActor :type Actor%20Object%20Reference) (OtherComp :type Primitive%20Component%20Object%20Reference) (OtherBodyIndex :type Integer) (bFromSweep :type Boolean) (SweepResult :type Hit%20Result%20Structure%20%28by%20ref%29))
  (Development|PrintString "right leg collider")
  (bind _asrobopart_right_leg (Utilities|Casting|CastToRobopartRightLeg OtherActor))
  (bind _output_get (Variables|Default|SetBaseRoboPart _asrobopart_right_leg))
  (Variables|Default|SetCollider (Variables|Default|GetRightLegPointCollider))
  (Development|PrintString "is right leg")
  (Class|BaseMagnetic|TriggerMagneticStop _output_get)
  (Variables|Default|SetPulling true))

(event EventTick
  (params (DeltaSeconds :type Float%20%28single-precision%29))
  (if (Variables|Default|GetPulling)
    (Development|PrintString "pulling")
    (bind _done (CallFunction|MovetoLocation (Transformation|GetWorldLocation (Variables|Default|GetCollider)) (Variables|Default|GetBaseRoboPart)))
    (Variables|Default|SetPulling (not _done))))

(fn ConstructionScript)

(fn MovetoLocation
  (params (TargetLocation :type Vector) (RoboPart :type Base%20Robo%20Part%20Object%20Reference))
  (bind _returnvalue (Transformation|GetActorLocation RoboPart))
  (bind _returnvalue_2 (Class|KismetMathLibrary|GetDirectionVector _returnvalue TargetLocation))
  (bind _returnvalue_3 (Math|Vector|VectorLength _returnvalue_2))
  (bind _output_get (LocalVariables|SetPercent (/ _returnvalue_3 (Variables|/Script/NewWorldDiscovery.BaseMagnetic|GetRotationPercentDistanceVelocity RoboPart))))
  (Development|PrintString (Utilities|String|ToString(Float) _returnvalue_3))
  (Physics|SetPhysicsLinearVelocity (Variables|/Script/NewWorldDiscovery.BaseMagnetic|GetMagneticMesh RoboPart) (* (* _returnvalue_2 (Variables|/Script/NewWorldDiscovery.BaseMagnetic|GetPullVelocity RoboPart)) _output_get) false "None")
  (return (<= _returnvalue_3 2.0)))