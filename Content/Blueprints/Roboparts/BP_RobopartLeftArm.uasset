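; BP_RobopartLeftArm is a robot left-arm part that plays dissolve effects when it spawns and when it is being destroyed.
; BeginPlay creates a dynamic M_RoboParts material on RoboMesh, then a timeline lowers DisolveStrength from full and clears the fringe.
; OnDestroying_Copy drives DisolveStrength from a second timeline, then resets it to zero and sets ReadyForDestroy, without destroying the actor itself.
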(event Custom|OnDestroying_Copy
  (bind _emissivepower (Timeline|Timeline_1 PlayFromStart)
    (:Update
      (Rendering|Material|SetScalarParameterValue (stale EventBeginPlay _returnvalue) "DisolveStrength" (Math|Float|Clamp(Float) _emissivepower) :!class /Script/Engine.MaterialInstanceDynamic))
    (:Finished
      (Rendering|Material|SetScalarParameterValue (stale EventBeginPlay _returnvalue) "DisolveStrength" 0.0 :!class /Script/Engine.MaterialInstanceDynamic)
      (Variables|Default|SetReadyForDestroy true)
      (Development|PrintString "Destroyed"))))

(event EventBeginPlay
  (bind _returnvalue (Rendering|Material|CreateDynamicMaterialInstance (Variables|Default|GetRoboMesh) 0 "/Game/MapElements/Materials/M_RoboParts.M_RoboParts" :!class /Script/Engine.PrimitiveComponent))
  (Rendering|Material|SetScalarParameterValue _returnvalue "FringeSize" 2.0 :!class /Script/Engine.MaterialInstanceDynamic)
  (Rendering|Material|SetScalarParameterValue _returnvalue "DisolveStrength" 1.0 :!class /Script/Engine.MaterialInstanceDynamic)
  (bind _emissivepower (Timeline|Timeline_0 PlayFromStart)
    (:Update
      (Rendering|Material|SetScalarParameterValue _returnvalue "DisolveStrength" (Math|Float|Clamp(Float) (- 1.0 _emissivepower)) :!class /Script/Engine.MaterialInstanceDynamic))
    (:Finished
      (Rendering|Material|SetScalarParameterValue _returnvalue "DisolveStrength" 0.0 :!class /Script/Engine.MaterialInstanceDynamic)
      (Rendering|Material|SetScalarParameterValue _returnvalue "FringeSize" 0.0 :!class /Script/Engine.MaterialInstanceDynamic))))

(fn ConstructionScript)